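; Test dummy character that serves as a lock-on target and damage receiver for the combat system.
; BeginPlay initializes its stats component and binds a health bar widget, which appears with the lock-on widget while targeted.
; Point damage prints the amount, reduces stats and plays impact effects; if a hit reaction is allowed, it sets the Disabled state and plays a montage.
; State manager checks report it untargetable and undamageable when Dead.
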(event EventBeginPlay
  (|CallParentFunction)
  (Default|InitializeStats (Variables|Default|GetStatsComponent))
  (bind _returnvalue (UserInterface|CreateWidget "/Game/CombatSystem/UI/WB_HealthBar.WB_HealthBar_C" (Game|GetPlayerController 0) (Variables|Default|GetStatsComponent) false))
  (UserInterface|SetWidget (Variables|Default|GetHealthBar) _returnvalue))

(event Collision|EventActorBeginOverlap
  (params (OtherActor :type Actor%20Object%20Reference)))

(event EventTick
  (params (DeltaSeconds :type Float%20%28single-precision%29)))

(event EventOnTargeted
  (params (bIsTargeted? :type Boolean))
  (Rendering|SetVisibility (Variables|Default|GetLockOnWidget) bIsTargeted? false)
  (Rendering|SetVisibility (Variables|Default|GetHealthBar) bIsTargeted? false))

(event Game|Damage|EventPointDamage
  (params (Damage :type Float%20%28single-precision%29) (DamageType :type Damage%20Type%20Object%20Reference) (HitLocation :type Vector :default "0, 0, 0") (HitNormal :type Vector :default "0, 0, 0") (HitComponent :type Primitive%20Component%20Object%20Reference) (BoneName :type Name :default "None") (ShotFromDirection :type Vector :default "0, 0, 0") (InstigatedBy :type Controller%20Object%20Reference) (DamageCauser :type Actor%20Object%20Reference) (HitInfo :type Hit%20Result%20Structure%20%28by%20ref%29))
  (Development|PrintString (Utilities|String|ToString(Float) Damage) true true "(R=1.000000,G=0.000000,B=0.101272,A=1.000000)")
  (Default|TakeDamage (Variables|Default|GetStatsComponent) Damage)
  (Audio|PlaySoundatLocation "/Game/CombatSystem/CourseFiles/SoundFX/Gruntling/A_Guardian_Impact_Cue.A_Guardian_Impact_Cue" HitLocation "0, 0, 0" 1.0 1.0 0.0 0 0 0 0)
  (Effects|SpawnEmitteratLocation 0 HitLocation)
  (if (CallFunction|CanReceiveHitReaction?)
    (Default|SetState (Variables|Default|GetBP_StateManagerComponent) "(TagName=\"Character.State.Disabled\")")
    (Animation|PlayAnimMontage "/Game/Characters/Mannequin_UE4/UE4_MannyAnims/Standing_React_Large_Front_Montage.Standing_React_Large_Front_Montage" 1.0 "None")))

(fn ConstructionScript
  (|CallParentFunction))

(fn CanReceiveDamage
  (return (not (Default|IsCurrentStateEqualtoAny? (Variables|Default|GetBP_StateManagerComponent) "(GameplayTags=((TagName=\"Character.State.Dead\")))"))))

(fn CanbeTargeted?
  (return (not (Default|IsCurrentStateEqualtoAny? (Variables|Default|GetBP_StateManagerComponent) "(GameplayTags=((TagName=\"Character.State.Dead\")))"))))