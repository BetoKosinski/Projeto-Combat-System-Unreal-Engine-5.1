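; BP_BaseWeapon is a base weapon item for melee combat, holding per-action montages, stat costs and damage multipliers.
; On equip it attaches to a hand or stowed socket, registers with the owner's combat component, updates the AnimInstance's combat type and configures its collision component.
; Collision hits apply point damage to valid receivers, scaled by the state manager's current action.
; It can also switch its mesh to simulated physics.
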(event OnHit(BP_CollisionComponent)
  (params (HitResult :type Hit%20Result%20Structure))
  (bind _hitactor (Collision|BreakHitResult HitResult))
  (bind _returnvalue (Class|CombatBPI|CanReceiveDamage(Message) _hitactor))
  (if _returnvalue
    (Game|Damage|ApplyPointDamage _hitactor (Stat|GetDamage) (Transformation|GetActorForwardVector (Components|GetOwner)) HitResult (Game|GetInstigatorController) self)))

(event Custom|SimulateWeaponPhysics
  (bind _returnvalue (CallFunction|GetItemMesh))
  (Collision|SetCollisionProfileName _returnvalue "PhysicsActor" true :!class /Script/Engine.PrimitiveComponent)
  (Physics|SetSimulatePhysics _returnvalue true))

(event EventBeginPlay
  (|CallParentFunction) ; This node is disabled and will not be called.\nDrag off pins to build functionality.
)

(event Collision|EventActorBeginOverlap
  (params (OtherActor :type Actor%20Object%20Reference))
  (|CallParentFunction OtherActor) ; This node is disabled and will not be called.\nDrag off pins to build functionality.
)

(event EventTick
  (params (DeltaSeconds :type Float%20%28single-precision%29))
  (|CallParentFunction DeltaSeconds) ; This node is disabled and will not be called.\nDrag off pins to build functionality.
)

(fn ConstructionScript
  (|CallParentFunction))

(fn OnEquipped
  (Variables|Default|SetCombatCombatComponent (Actor|GetComponentbyClass (Components|GetOwner) "/Game/CombatSystem/Blueprints/Components/BP_CombatComponent.BP_CombatComponent_C"))
  (Variables|Default|SetOwnerStateManager (Actor|GetComponentbyClass (Components|GetOwner) "/Game/CombatSystem/Blueprints/Components/BP_StateManagerComponent.BP_StateManagerComponent_C"))
  (CallFunction|AttachActor (select (Default|IsCombatEnabled? (Variables|Default|GetCombatCombatComponent)) (Variables|Initialization|GetHandSocketName) (Variables|Default|GetAttach%20Socket%20Name)))
  (Default|SetMainWeapon (Variables|Default|GetCombatCombatComponent) self)
  (Class|AnimInstanceBPI|UpdateCombatType(Message) (Components|SkeletalMesh|GetAnimInstance (Variables|/Script/Engine.Character|GetMesh (.AsCharacter (Utilities|Casting|CastToCharacter (Components|GetOwner))))) (Variables|Initialization|GetCombatType))
  (Default|SetCollisionMesh (Variables|Default|GetBP_CollisionComponent) (CallFunction|GetItemMesh))
  (Default|AddActortoIgnore (Variables|Default|GetBP_CollisionComponent) (Components|GetOwner)))

(fn GetActionMontages
  (params (CharacterAction :type Gameplay%20Tag%20Structure))
  (|SwitchGameplayTag CharacterAction
    (:Character.Action.Attack.Light%20Attack
      (return (Variables|Montages|GetLightAttackMontages)))
    (:Character.Action.Attack.Heavy%20Attack
      (return (Variables|Montages|GetHeavyAttackMontages)))
    (:Character.Action.Attack.Sprint%20Attack
      (return (Variables|Montages|GetSprinting%20Attack%20Montages)))
    (:Character.Action.Attack.Charged%20Attack
      (return (Variables|Montages|GetCharged%20Attack%20Montages)))
    (:Character.Action.Attack.Falling%20Attack
      (return (Variables|Montages|GetFalling%20Attack%20Montages)))
    (:Character.Action.Dodge
      (return (Variables|Montages|GetDodgeMontages)))
    (:Character.Action.Enter%20Combat
      (return (Utilities|Array|MakeArray (Variables|Montages|GetEnterCombat))))
    (:Character.Action.Exit%20Combat
      (return (Utilities|Array|MakeArray (Variables|Montages|GetExitCombat))))))

(fn GetStatCostforAction
  (bind _ownerstatemanager (Variables|Default|GetOwnerStateManager)
    (:then
      (return (.Value (Utilities|Map|Find (Variables|Stat|GetActionStatCost) (Default|GetCurrentAction _ownerstatemanager)))))
    (:else
      (return 0.0))))

(fn GetDamage
  (bind _ownerstatemanager (Variables|Default|GetOwnerStateManager)
    (:then
      (return (* (Variables|Stat|GetDamage) (Math|Float|Clamp(Float) (.Value (Utilities|Map|Find (Variables|Stat|GetActionDamageMultiplier) (Default|GetCurrentAction _ownerstatemanager))) 1.0 (.Value (Utilities|Map|Find (Variables|Stat|GetActionDamageMultiplier) (Default|GetCurrentAction _ownerstatemanager)))))))
    (:else
      (return (Variables|Stat|GetDamage)))))