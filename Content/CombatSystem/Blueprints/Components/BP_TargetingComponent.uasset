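; Character component that provides toggleable combat lock-on, keeping the controller aimed at a targeted actor.
; Finds targets by sphere tracing along the camera's forward vector for TargetingBPI implementers, notifying them when targeting changes.
; Each tick it interpolates control pitch and yaw toward the target, unlocking when CanTargetActor fails.
; Lock toggles also switch movement to camera-oriented rotation, depending on BP_CombatComponent state and speed mode, otherwise using the default mode.
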(event Custom|Enable%20Lock%20On
  (bind (_returnvalu _foundtarget) (CallFunction|FindTarget))
  (if (and _returnvalu (CallFunction|CanTargetActor? _foundtarget))
    (CallFunction|SetTargetActor _foundtarget)
    (CallFunction|SetIsTargeting true)
    (CallFunction|UpdateRotationMode)))

(event Custom|Disable%20Lock%20On
  (CallFunction|SetIsTargeting false)
  (CallFunction|SetTargetActor)
  (CallFunction|UpdateRotationMode))

(event Custom|Toggle%20Lock%20On
  (if (not (CallFunction|IsTargeting?))
    (CallFunction|EnableLockon)
    (else
      (CallFunction|DisableLockon))))

(event EventBeginPlay
  (bind _ascharacter (Utilities|Casting|CastToCharacter (Components|GetOwner)))
  (Variables|Default|SetOwner%20Character _ascharacter)
  (Variables|Default|SetOwnerController (Pawn|GetController (Variables|Default|GetOwner%20Character)))
  (Variables|Default|SetFollowCamera (Actor|GetComponentbyClass (Variables|Default|GetOwner%20Character) "/Script/Engine.CameraComponent")))

(event EventTick
  (params (DeltaSeconds :type Float%20%28single-precision%29))
  (if (Variables|Default|GetbIsTargeting)
    (CallFunction|UpdateTargetingControlLocation)))

(fn SetIsTargeting
  (params (bEnableTargeting :type Boolean))
  (Variables|Default|SetbIsTargeting bEnableTargeting)
  (bind _target_actor (Variables|Default|GetTarget%20Actor)
    (:then
      (Class|TargetingBPI|OnTargeted(Message) _target_actor bEnableTargeting))
    (:else)))

(fn IsTargeting?
  (return (Variables|Default|GetbIsTargeting)))

(fn FindTarget
  (bind (_outhit _returnvalue) (Collision|SphereTraceForObjects (Transformation|GetActorLocation (Components|GetOwner)) (+ (* (Math|Vector|GetForwardVector (Variables|Default|GetFollowCamera)) (Variables|Initialize|GetTargetingDistance)) (Transformation|GetActorLocation (Components|GetOwner))) (Variables|Initialize|GetTargeting%20Radius) (Variables|Initialize|GetTarget%20Object%20Types) false (Utilities|Array|MakeArray (Components|GetOwner)) "None"))
  (if (and _returnvalue (Utilities|IsValid (.HitActor (Collision|BreakHitResult _outhit))))
    (if (Utilities|DoesObjectImplementInterface (.HitActor (Collision|BreakHitResult _outhit)) "/Game/CombatSystem/Blueprints/Interfaces/TargetingBPI.TargetingBPI_C")
      (return true (.HitActor (Collision|BreakHitResult _outhit)))
      (else
        (return false 0)))
    (else
      (return false 0))))

(fn SetTargetActor
  (params (New%20Target%20Actor :type Actor%20Object%20Reference))
  (Variables|Default|SetTarget%20Actor New%20Target%20Actor))

(fn GetTargetActor
  (return (Variables|Default|GetTarget%20Actor)))

(fn UpdateTargetingControlLocation
  (bind _returnvalue (Utilities|Time|GetWorldDeltaSeconds))
  (bind _returnvalue_2 (Components|GetOwner))
  (bind _ownercontroller (Variables|Default|GetOwnerController))
  (bind _target_actor (Variables|Default|GetTarget%20Actor))
  (bind _target_rotation_interp_speed (Variables|Initialize|GetTarget%20Rotation%20Interp%20Speed))
  (bind _returnvalue_3 (Transformation|GetActorRotation _ownercontroller))
  (bind _returnvalue_4 (Transformation|GetActorLocation _returnvalue_2))
  (bind _returnvalue_5 (Transformation|GetActorLocation _target_actor))
  (bind _returnvalue_6 (- _returnvalue_5 "0.000000,0.000000,100.000000"))
  (bind _returnvalue_7 (Math|Rotator|FindLookatRotation _returnvalue_4 _returnvalue_6))
  (bind _returnvalue_8 (Math|Interpolation|RInterpTo _returnvalue_3 _returnvalue_7 _returnvalue _target_rotation_interp_speed))
  (if (and (Utilities|IsValid (Variables|Default|GetOwnerController)) (Utilities|IsValid (Variables|Default|GetTarget%20Actor)))
    (if (CallFunction|CanTargetActor? (Variables|Default|GetTarget%20Actor))
      (Pawn|SetControlRotation (Variables|Default|GetOwnerController) (Math|Rotator|MakeRotator (.Roll (Math|Rotator|BreakRotator _returnvalue_3)) (.pitch _returnvalue_8) (.yaw _returnvalue_8)))
      (else
        (CallFunction|DisableLockon)))))

(fn SetRotationMode
  (params (NewRotationMode :type E_RotationMode%20Enum :default "NewEnumerator0"))
  (bind _owner_character (Variables|Default|GetOwner%20Character))
  (bind _charactermovement (Variables|/Script/Engine.Character|GetCharacterMovement _owner_character))
  (bind _output_get (Variables|Default|SetCurrent%20Rotation%20Mode NewRotationMode))
  (switch Utilities|FlowControl|Switch|SwitchonE_RotationMode _output_get
    (:NewEnumerator0
      (Variables|/Script/Engine.Pawn|SetbUseControllerRotationYaw _owner_character false)
      (Variables|/Script/Engine.CharacterMovementComponent|SetbUseControllerDesiredRotation _charactermovement true)
      (Variables|/Script/Engine.CharacterMovementComponent|SetbOrientRotationToMovement _charactermovement false))
    (:NewEnumerator1
      (Variables|/Script/Engine.Pawn|SetbUseControllerRotationYaw _owner_character false)
      (Variables|/Script/Engine.CharacterMovementComponent|SetbUseControllerDesiredRotation _charactermovement false)
      (Variables|/Script/Engine.CharacterMovementComponent|SetbOrientRotationToMovement _charactermovement true))))

(fn GetRotationMode
  (return (Variables|Default|GetCurrent%20Rotation%20Mode)))

(fn CanTargetActor?
  (params (InTargetActor :type Actor%20Object%20Reference))
  (Utilities|IsValid InTargetActor
    (:Is%20Valid
      (bind _returnvalue (Class|TargetingBPI|CanbeTargeted?(Message) InTargetActor))
      (return (and _returnvalue (< (Transformation|GetDistanceTo (Components|GetOwner) (Variables|Default|GetTarget%20Actor)) (Variables|Initialize|GetTargetingDistance)))))
    (:Is%20Not%20Valid
      (return false))))

(fn UpdateRotationMode
  (Utilities|IsValid (Variables|Default|GetOwnerCombatComponent)
    (:Is%20Valid
      _)
    (:Is%20Not%20Valid
      (Variables|Default|SetOwnerCombatComponent (Actor|GetComponentbyClass (Variables|Default|GetOwner%20Character) "/Game/CombatSystem/Blueprints/Components/BP_CombatComponent.BP_CombatComponent_C"))))
  (bind _returnvalue (Class|CombatBPI|GetMovementSpeedMode(Message) (Variables|Default|GetOwner%20Character)))
  (CallFunction|SetRotationMode (select (Math|Boolean|ANDBoolean (Default|IsCombatEnabled? (Variables|Default|GetOwnerCombatComponent)) (Utilities|Enum|NotEqual(Enum) _returnvalue "NewEnumerator2") (CallFunction|IsTargeting?)) "NewEnumerator0" (Variables|Initialize|GetDefault%20Rotation%20Mode))))